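; BP_Balling is a resettable six-bottle setup, apparently for a bowling or knock-down minigame.
; When the player pawn overlaps the Reset component, a 0.2-second retriggerable delay runs before ResetBottle fires.
; ResetBottle teleports each bottle to the world transform of its matching reference component (R1 to R6), without sweeping.
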(event `Reset Bottle`
  ;[1 1 1] Reset bottles
  (`|ExecutionSequence`
    (:`then_0`
      (`SceneComponent.K2_SetWorldTransform` (`self.Bottle1`) (`SceneComponent.K2_GetComponentToWorld` (`self.R1`)) false true))
    (:`then_1`
      (`SceneComponent.K2_SetWorldTransform` (`self.Bottle2`) (`SceneComponent.K2_GetComponentToWorld` (`self.R2`)) false true))
    (:`then_2`
      (`SceneComponent.K2_SetWorldTransform` (`self.Bottle3`) (`SceneComponent.K2_GetComponentToWorld` (`self.R3`)) false true))
    (:`then_3`
      (`SceneComponent.K2_SetWorldTransform` (`self.Bottle4`) (`SceneComponent.K2_GetComponentToWorld` (`self.R4`)) false true))
    (:`then_4`
      (`SceneComponent.K2_SetWorldTransform` (`self.Bottle5`) (`SceneComponent.K2_GetComponentToWorld` (`self.R5`)) false true))
    (:`then_5`
      (`SceneComponent.K2_SetWorldTransform` (`self.Bottle6`) (`SceneComponent.K2_GetComponentToWorld` (`self.R6`)) false true))))

(event `self.Reset.OnComponentBeginOverlap`
  (params (OverlappedComponent :type "PrimitiveComponent Object Reference") (OtherActor :type "Actor Object Reference") (OtherComp :type "PrimitiveComponent Object Reference") (OtherBodyIndex :type Integer) (bFromSweep :type Boolean) (SweepResult :type "HitResult Structure (by ref)"))
  (if (== OtherActor (`GameplayStatics.GetPlayerPawn` 0))
    (`KismetSystemLibrary.RetriggerableDelay` 0.2)
    (`self.Reset Bottle`)))

(fn `UserConstructionScript`)
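; BP_NPC is a non-player character that shows a floating line of text when the player overlaps its Box trigger.
; The construction script picks the male or female mannequin from Gender and fills in the NPC's text.
; Tick turns visible text to match the player camera's rotation, and retriggerable delays time its hiding.
; On the first showing only, the player character displays its TextPlayer reply after a short delay.
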(event `self.ReceiveBeginPlay`
  (bind _asbp_top_down_character (cast `/Game/Character/Blueprints/BP_TopDownCharacter` (`GameplayStatics.GetPlayerPawn` 0)))
  (set `self.PlayerRef` _asbp_top_down_character))

(event `self.ReceiveTick`
  (params (DeltaSeconds :type "Float (single-precision)"))
  ;[1 1 1] Set TextRender facing towards camera
  (if (`SceneComponent.IsVisible` (`self.TextRender`))
    (`SceneComponent.K2_SetWorldRotation` (`self.TextRoot`) (`SceneComponent.K2_GetComponentRotation` (`/Game/Character/Blueprints/BP_TopDownCharacter.Camera1` (`self.PlayerRef`))) false false)))

(event `self.Box.OnComponentBeginOverlap`
  (params (OverlappedComponent :type "PrimitiveComponent Object Reference") (OtherActor :type "Actor Object Reference") (OtherComp :type "PrimitiveComponent Object Reference") (OtherBodyIndex :type Integer) (bFromSweep :type Boolean) (SweepResult :type "HitResult Structure (by ref)"))
  ;[1 1 1] Text Events
  (if (== OtherActor (`self.PlayerRef`))
    (`self.ShowText`)))

(event `self.ShowText`
  (bind _playerref (`self.PlayerRef`))
  ;[1 1 1] Text Events
  (`SceneComponent.SetVisibility` (`self.TextRender`) true false)
  (`|ExecutionSequence`
    (:`then_0`
      (`KismetSystemLibrary.RetriggerableDelay` 5.0)
      (`SceneComponent.SetVisibility` (`self.TextRender`) false false))
    (:`then_1`
      (`/Engine/EditorBlueprintResources/StandardMacros.DoOnce` false
        (:`Completed`
          (`KismetSystemLibrary.RetriggerableDelay` 2.0)
          (`self.ShowText` _playerref)
          (`self.SetText` _playerref (`self.Text_Player`)))))))

(event `self.SetText`
  (params (Text :type Text))
  ;[1 1 1] Text Events
  (`TextRenderComponent.K2_SetText` (`self.TextRender`) Text))

(fn `UserConstructionScript`
  (bind _mesh (`self.Mesh`))
  (`|ExecutionSequence`
    (:`then_0`
      (if (`self.Gender`)
        (`SkinnedMeshComponent.SetSkinnedAssetAndUpdate` _mesh "/Game/Character/Mannequin/Mesh/SK_Mannequin_Female.SK_Mannequin_Female" true)
        (else
          (`SkinnedMeshComponent.SetSkinnedAssetAndUpdate` _mesh "/Game/Character/Mannequin/Mesh/SK_Mannequin.SK_Mannequin" true))))
    (:`then_1`
      (`TextRenderComponent.K2_SetText` (`self.TextRender`) (`self.Text_NPC`)))))
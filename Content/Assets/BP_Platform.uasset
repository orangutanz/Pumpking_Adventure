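; BP_Platform is a moving platform that shuttles back and forth between its placed transform and an offset target.
; The construction script stores the actor transform as Origin and builds the target by adding world-space offsets on the enabled X, Y and Z axes.
; Tick moves an alpha up or down by MoveRate, flips direction past 0 or 1, and sets the root to the interpolated transform without sweeping.
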(event `self.ReceiveBeginPlay`)

(event `self.ReceiveTick`
  (params (DeltaSeconds :type "Float (single-precision)"))
  (bind _reversablealpha (`self.ReversableAlpha`))
  (bind _defaultsceneroot (`self.DefaultSceneRoot`))
  (`|ExecutionSequence`
    (:`then_0`
      ;[1 1 1] Comment
      (if (> _reversablealpha 1.0)
        (set `self.OriginToTarget` false)
        (elif (< _reversablealpha 0.0)
          (set `self.OriginToTarget` true))))
    (:`then_2`
      (if (`self.OriginToTarget`)
        ;[1 1 1] Set Alpha to Target
        (bind _output_get (set `self.ReversableAlpha` (+ (`self.ReversableAlpha`) (* (`GameplayStatics.GetWorldDeltaSeconds`) (`self.MoveRate`)))))
        (`SceneComponent.K2_SetWorldTransform` _defaultsceneroot (`KismetMathLibrary.TLerp` (`self.Origin`) (`self.Traget`) _output_get) false false)
        (else
          ;[1 1 1] Set Alpha to Origin
          (bind _output_get_2 (set `self.ReversableAlpha` (- (`self.ReversableAlpha`) (* (`GameplayStatics.GetWorldDeltaSeconds`) (`self.MoveRate`)))))
          (`SceneComponent.K2_SetWorldTransform` _defaultsceneroot (`KismetMathLibrary.TLerp` (`self.Origin`) (`self.Traget`) _output_get_2) false false))))))

(fn `UserConstructionScript`
  (bind (_traget_location _traget_rotation _traget_scale) (`KismetMathLibrary.BreakTransform` (`self.Traget`)))
  (bind _returnvalue (`KismetMathLibrary.TransformLocation` (`self.Traget`)))
  (bind _output_get (set `self.Origin` (`self.GetTransform`)))
  (set `self.Traget` (`KismetMathLibrary.MakeTransform` (.location _output_get) (.rotation _output_get) (.scale _output_get)))
  (`|ExecutionSequence`
    (:`then_0`
      (if (`self.AxisZ`)
        (set `self.Traget` (`KismetMathLibrary.MakeTransform` (+ _returnvalue (`KismetMathLibrary.MakeVector` 0.0 0.0 (`self.Offset_Z`))) _traget_rotation _traget_scale))))
    (:`then_1`
      (if (`self.AxisX`)
        (set `self.Traget` (`KismetMathLibrary.MakeTransform` (+ _returnvalue (`KismetMathLibrary.MakeVector` (`self.Offset_X`))) _traget_rotation _traget_scale))))
    (:`then_2`
      (if (`self.AxisY`)
        (set `self.Traget` (`KismetMathLibrary.MakeTransform` (+ _returnvalue (`KismetMathLibrary.MakeVector` 0.0 (`self.Offset_Y`))) _traget_rotation _traget_scale))))))
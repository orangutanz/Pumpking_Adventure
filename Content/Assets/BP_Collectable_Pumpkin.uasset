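; Collectable pumpkin actor that the player gathers by hitting it with a projectile in a top-down game.
; Construction picks one of three pumpkin meshes at random and reads a cel shader from a data table into a variable.
; On BeginPlay it raises the player's collectable maximum.
; The first projectile overlap disables collision, plays a random squash sound, destroys the actor after a short delay, increments the player's count and prints progress.
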(event `self.ReceiveBeginPlay`
  (bind _asbp_top_down_character (cast `/Game/Character/Blueprints/BP_TopDownCharacter` (`GameplayStatics.GetPlayerPawn` 0)))
  (bind _output_get (set `self.TopDownPlayerPawn` _asbp_top_down_character))
  (set `/Game/Character/Blueprints/BP_TopDownCharacter.CollectableMax` (+ (`/Game/Character/Blueprints/BP_TopDownCharacter.CollectableMax` _output_get) 1) _output_get))

(event `self.StaticMesh.OnComponentBeginOverlap`
  (params (OverlappedComponent :type "PrimitiveComponent Object Reference") (OtherActor :type "Actor Object Reference") (OtherComp :type "PrimitiveComponent Object Reference") (OtherBodyIndex :type Integer) (bFromSweep :type Boolean) (SweepResult :type "HitResult Structure (by ref)"))
  (bind _topdownplayerpawn (`self.TopDownPlayerPawn`))
  (bind _topdownplayerpawn_2 (`self.TopDownPlayerPawn`))
  (cast `/Game/Character/Blueprints/BP_Projectile` OtherActor)
  (`/Engine/EditorBlueprintResources/StandardMacros.DoOnce` false
    (:`Completed`
      (`self.SetActorEnableCollision` false)
      (if (>= (`KismetMathLibrary.RandomIntegerInRange` 0 2) 1)
        (`GameplayStatics.PlaySound2D` "/Game/Audio/Effect/squash.squash" 1.0 1.0 0.0 null null)
        (else
          (`GameplayStatics.PlaySound2D` "/Game/Audio/Effect/squash2.squash2" 1.0 1.0 0.0 null null)))
      (`KismetSystemLibrary.Delay` 0.1)
      (`self.K2_DestroyActor`)
      (set `/Game/Character/Blueprints/BP_TopDownCharacter.CollectableCount` (+ (`/Game/Character/Blueprints/BP_TopDownCharacter.CollectableCount` _topdownplayerpawn_2) 1) _topdownplayerpawn_2)
      (`KismetSystemLibrary.PrintString` (`KismetStringLibrary.Concat_StrStr` "Collected " (`KismetStringLibrary.Concat_StrStr` (`KismetStringLibrary.Concat_StrStr` (`KismetStringLibrary.Conv_IntToString` (`/Game/Character/Blueprints/BP_TopDownCharacter.CollectableCount` _topdownplayerpawn)) " out of ") (`KismetStringLibrary.Conv_IntToString` (`/Game/Character/Blueprints/BP_TopDownCharacter.CollectableMax` _topdownplayerpawn))))))))

(fn `UserConstructionScript`
  (bind _returnvalue (`KismetMathLibrary.RandomIntegerInRange` 0 3))
  (bind _staticmesh (`self.StaticMesh`))
  (bind (_datatable _rowname) (break `DataTableRowHandle` (`self.ShaderTypeSelector`)))
  (`|ExecutionSequence`
    (:`then_0`
      (if (and (>= _returnvalue 0) (< _returnvalue 1))
        (`StaticMeshComponent.SetStaticMesh` _staticmesh "/Game/Addons/AdvancedVillagePack/Meshes/SM_Pumpkin_Var01.SM_Pumpkin_Var01")
        (elif (and (>= _returnvalue 1) (< _returnvalue 2))
          (`StaticMeshComponent.SetStaticMesh` _staticmesh "/Game/Addons/AdvancedVillagePack/Meshes/SM_Pumpkin_Var02.SM_Pumpkin_Var02")
          (else
            (`StaticMeshComponent.SetStaticMesh` _staticmesh "/Game/Addons/AdvancedVillagePack/Meshes/SM_Pumpkin_Var03.SM_Pumpkin_Var03")))))
    (:`then_1`
      (bind _returnvalue_2 (`|GetDataTableRow` _datatable _rowname)
        (:`then`
          (set `self.CelShaderInstance` (`.CelShader_2_216C332B4322A65A1CC616BD1C0C153A` (break `/Game/Geometry/Misc/ST_CelShaderType` _returnvalue_2))))))))
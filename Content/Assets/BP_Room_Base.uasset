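; Base room actor that builds itself from data-table mesh choices and hides its roof or floor when the player is inside or underneath.
; The construction script sets roof, floor and two wall meshes, flagging roof or floor as absent for "NoMesh" rows.
; Inside and under trigger boxes call SetSeethrough, which toggles visibility and collision.
; Retriggerable delays precede restoring the roof on leaving inside and the floor on leaving underneath.
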(event `self.BoxCollider_in.OnComponentBeginOverlap`
  (params (OverlappedComponent :type "PrimitiveComponent Object Reference") (OtherActor :type "Actor Object Reference") (OtherComp :type "PrimitiveComponent Object Reference") (OtherBodyIndex :type Integer) (bFromSweep :type Boolean) (SweepResult :type "HitResult Structure (by ref)"))
  ;[1 1 1] Trigger inside
  (if (== OtherActor (`GameplayStatics.GetPlayerPawn` 0))
    (`self.SetSeethrough` (`self.Roof`) true)))

(event `self.BoxCollider_in.OnComponentEndOverlap`
  (params (OverlappedComponent :type "PrimitiveComponent Object Reference") (OtherActor :type "Actor Object Reference") (OtherComp :type "PrimitiveComponent Object Reference") (OtherBodyIndex :type Integer))
  ;[1 1 1] Trigger inside
  (if (== (`GameplayStatics.GetPlayerPawn` 0) OtherActor)
    (`KismetSystemLibrary.RetriggerableDelay` 0.2)
    (`self.SetSeethrough` (`self.Roof`))))

(event `self.BoxCollider_under.OnComponentBeginOverlap`
  (params (OverlappedComponent :type "PrimitiveComponent Object Reference") (OtherActor :type "Actor Object Reference") (OtherComp :type "PrimitiveComponent Object Reference") (OtherBodyIndex :type Integer) (bFromSweep :type Boolean) (SweepResult :type "HitResult Structure (by ref)"))
  ;[1 1 1] Triiger under
  (if (== OtherActor (`GameplayStatics.GetPlayerPawn` 0))
    (`|ExecutionSequence`
      (:`then_0`
        (if (`self.HasFloor`)
          (`self.SetSeethrough` (`self.Floor`) true)))
      (:`then_1`
        (if (`self.HasRoof`)
          (`self.SetSeethrough` (`self.Roof`) true))))))

(event `self.ReceiveBeginPlay`
  (`|ExecutionSequence`
    (:`then_0`
      (if (not (`self.HasRoof`))
        (`self.SetSeethrough` (`self.Roof`) true)))
    (:`then_1`
      (if (not (`self.HasFloor`))
        (`self.SetSeethrough` (`self.Floor`) true)))))

(event `self.BoxCollider_under.OnComponentEndOverlap`
  (params (OverlappedComponent :type "PrimitiveComponent Object Reference") (OtherActor :type "Actor Object Reference") (OtherComp :type "PrimitiveComponent Object Reference") (OtherBodyIndex :type Integer))
  ;[1 1 1] Triiger under
  (if (== (`GameplayStatics.GetPlayerPawn` 0) OtherActor)
    (`|ExecutionSequence`
      (:`then_0`
        (if (`self.HasFloor`)
          (`KismetSystemLibrary.RetriggerableDelay` 0.2)
          (`self.SetSeethrough` (`self.Floor`))))
      (:`then_1`
        (if (`self.HasRoof`)
          (`self.SetSeethrough` (`self.Roof`)))))))

(fn `SetSeethrough`
  (params (Mesh :type "StaticMeshComponent Object Reference") (CanSeeThrough :type Boolean))
  (if CanSeeThrough
    (`PrimitiveComponent.SetCollisionEnabled` Mesh "NoCollision")
    (`SceneComponent.SetVisibility` Mesh false false)
    (else
      (`PrimitiveComponent.SetCollisionEnabled` Mesh "QueryOnly")
      (`SceneComponent.SetVisibility` Mesh true false))))

(fn `SetUp`)

(fn `UserConstructionScript`
  (bind _roof (`self.Roof`))
  (bind _floor (`self.Floor`))
  (bind (_datatable _rowname) (break `DataTableRowHandle` (`self.RoofType`)))
  (bind (_datatable_2 _rowname_2) (break `DataTableRowHandle` (`self.FloorType`)))
  (bind (_datatable_3 _rowname_3) (break `DataTableRowHandle` (`self.Wall_NE_Type`)))
  (bind (_datatable_4 _rowname_4) (break `DataTableRowHandle` (`self.Wall_SW_Type`)))
  (`|ExecutionSequence`
    (:`then_0`
      (if (!= _rowname "NoMesh")
        (bind _returnvalue (`|GetDataTableRow` _datatable _rowname)
          (:`then`
            (`StaticMeshComponent.SetStaticMesh` _roof (`.Mesh_2_4BB4B10A4299EA302529C7BE10D6EA8C` (break `/Game/Geometry/Misc/ST_BuildingMeshType` _returnvalue))) ; Set Roof Mesh
          ))
        (else
          (`StaticMeshComponent.SetStaticMesh` _roof "/Game/Geometry/Meshes/1M_Cube.1M_Cube") ; Set Roof Mesh
          (`SceneComponent.SetVisibility` _roof false false)
          (set `self.HasRoof` false)
          (`PrimitiveComponent.SetCollisionEnabled` (`self.BoxCollider_in`) "NoCollision")
          (`PrimitiveComponent.SetCollisionEnabled` _roof "NoCollision"))))
    (:`then_1`
      (if (!= _rowname_2 "NoMesh")
        (bind _returnvalue_2 (`|GetDataTableRow` _datatable_2 _rowname_2)
          (:`then`
            (`StaticMeshComponent.SetStaticMesh` _floor (`.Mesh_2_4BB4B10A4299EA302529C7BE10D6EA8C` (break `/Game/Geometry/Misc/ST_BuildingMeshType` _returnvalue_2))) ; Set Floor Mesh
          ))
        (else
          (`StaticMeshComponent.SetStaticMesh` _floor "/Game/Geometry/Meshes/1M_Cube.1M_Cube")
          (`PrimitiveComponent.SetCollisionEnabled` _floor "NoCollision")
          (`SceneComponent.SetVisibility` _floor false false)
          (set `self.HasFloor` false))))
    (:`then_2`
      (bind _returnvalue_3 (`|GetDataTableRow` _datatable_4 _rowname_4)
        (:`then`
          (`StaticMeshComponent.SetStaticMesh` (`self.Wall_SW`) (`.Mesh_2_4BB4B10A4299EA302529C7BE10D6EA8C` (break `/Game/Geometry/Misc/ST_BuildingMeshType` _returnvalue_3))))))
    (:`then_3`
      (bind _returnvalue_4 (`|GetDataTableRow` _datatable_3 _rowname_3)
        (:`then`
          (`StaticMeshComponent.SetStaticMesh` (`self.Wall_NE`) (`.Mesh_2_4BB4B10A4299EA302529C7BE10D6EA8C` (break `/Game/Geometry/Misc/ST_BuildingMeshType` _returnvalue_4))))))))
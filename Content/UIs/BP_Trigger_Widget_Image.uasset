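; Trigger volume actor that shows an on-screen image, apparently mouse or keyboard info, while the player stands in it.
; When the player pawn enters CollisionBox, it creates UI_MouseInfo and/or UI_KeyInfo per the ImageMouse and ImageKeyboard flags, applies DisplayImage and adds them to the viewport.
; End overlap removes the flagged widgets without checking which actor left.
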(event `self.CollisionBox.OnComponentEndOverlap`
  (params (OverlappedComponent :type "PrimitiveComponent Object Reference") (OtherActor :type "Actor Object Reference") (OtherComp :type "PrimitiveComponent Object Reference") (OtherBodyIndex :type Integer))
  (`|ExecutionSequence`
    (:`then_0`
      (if (`self.Image_Mouse`)
        ;[1 1 1] Remove
        (`Widget.RemoveFromParent` (stale `self.CollisionBox.OnComponentBeginOverlap` _returnvalue))))
    (:`then_1`
      (if (`self.Image_Keyboard`)
        (`Widget.RemoveFromParent` (stale `self.CollisionBox.OnComponentBeginOverlap` _returnvalue_2))))))

(event `self.CollisionBox.OnComponentBeginOverlap`
  (params (OverlappedComponent :type "PrimitiveComponent Object Reference") (OtherActor :type "Actor Object Reference") (OtherComp :type "PrimitiveComponent Object Reference") (OtherBodyIndex :type Integer) (bFromSweep :type Boolean) (SweepResult :type "HitResult Structure (by ref)"))
  (bind _display_image (`self.Display_Image`))
  (if (== OtherActor (`GameplayStatics.GetPlayerPawn` 0))
    (`|ExecutionSequence`
      (:`then_0`
        (if (`self.Image_Mouse`)
          ;[1 1 1] Create
          (bind _returnvalue (`|CreateWidget` "/Game/UIs/UI_MouseInfo.UI_MouseInfo_C"))
          (`Image.SetBrushFromTexture` (`/Game/UIs/UI_MouseInfo.Image` _returnvalue) _display_image false)
          (`UserWidget.AddToViewport` _returnvalue 0)))
      (:`then_1`
        (if (`self.Image_Keyboard`)
          (bind _returnvalue_2 (`|CreateWidget` "/Game/UIs/UI_KeyInfo.UI_KeyInfo_C"))
          (`Image.SetBrushFromTexture` (`/Game/UIs/UI_KeyInfo.Image` _returnvalue_2) _display_image false)
          (`UserWidget.AddToViewport` _returnvalue_2 0))))))

(fn `UserConstructionScript`)